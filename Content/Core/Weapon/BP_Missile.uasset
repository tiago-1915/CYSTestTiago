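; BP_Missile is a networked missile projectile that explodes on hit, or after a timeout, and damages nearby players.
; The server briefly delays enabling collision, records the first impact or timeout point in Hit, then destroys the actor after a delay.
; OnRep_Hit plays explosion effects and, on authority, sphere-traces for unique BP_Players to damage.
; The distance-based damage mapping has identical output bounds, so damage is flat.
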(event OnComponentHit(Sphere)
  (params (HitComponent :type Primitive%20Component%20Object%20Reference) (OtherActor :type Actor%20Object%20Reference) (OtherComp :type Primitive%20Component%20Object%20Reference) (NormalImpulse :type Vector :default "0, 0, 0") (Hit :type Hit%20Result%20Structure%20%28by%20ref%29))
  ;[1 1 1] Hit Event
  (Networking|SwitchHasAuthority
    (:Authority
      (if (not (Variables|Default|GetHitEvent))
        (Variables|Default|SetHitEvent true)
        (Variables|Default|SetHit Hit)
        ;[1 1 1] Destroy Actor
        (Utilities|FlowControl|Delay 5.0)
        (Actor|DestroyActor)))))

(event EventBeginPlay
  (bind _sphere (Variables|Default|GetSphere))
  (bind _returnvalue (Transformation|GetWorldLocation _sphere))
  ;[1 1 1] Time Auto Destroy
  (Networking|SwitchHasAuthority
    (:Authority
      (Utilities|FlowControl|Sequence
        (:then_0
          (Utilities|FlowControl|Delay 0.1)
          (Collision|SetCollisionEnabled (Variables|Default|GetSphere) "QueryAndPhysics"))
        (:then_1
          (Utilities|FlowControl|Delay 1e+01)
          (if (not (Variables|Default|GetHitEvent))
            (Variables|Default|SetHitEvent true)
            (Variables|Default|SetHit (Collision|MakeHitResult false false 0.0 0.0 _returnvalue _returnvalue "0,0,1" "0,0,1" 0 0))
            ;[1 1 1] Destroy Actor
            (Utilities|FlowControl|Delay 5.0)
            (Actor|DestroyActor)))))))

(fn ConstructionScript)

(fn OnRepHit
  (bind _returnvalue (Math|Float|MakeLiteralFloat 5e+02))
  (bind _hit (Variables|Default|GetHit))
  (bind _hit_2 (Variables|Default|GetHit))
  (bind _impactpoint (Collision|BreakHitResult _hit))
  (bind _impactpoint_2 (Collision|BreakHitResult _hit_2))
  ;[1 1 1] Spawn Emmiter And Sound Hit
  (Components|DestroyComponent (Variables|Default|GetStaticMesh))
  (Effects|SpawnEmitteratLocation "/Game/Assets/Realistic_Starter_VFX_Pack_Vol2/Particles/Explosion/P_Explosion_Big_B.P_Explosion_Big_B" _impactpoint_2 "0, 0, 0" "3.000000,3.000000,3.000000")
  (Audio|SpawnSoundatLocation "/Game/Assets/MilitaryWeapSilverSound/Sound/RocketLauncher/Cues/RocketLauncher_Explosion_Cue.RocketLauncher_Explosion_Cue" _impactpoint_2 "0, 0, 0" 1.0 1.0 0.0 0 0)
  (Components|Activation|Deactivate (Variables|Default|GetParticleSystem))
  (Networking|SwitchHasAuthority
    (:Authority
      ;[1 1 1] Find Player Hit Area
      (bind _outhits (Collision|MultiSphereTraceForObjects _impactpoint (+ _impactpoint "0.000000,0.000000,1.000000") _returnvalue (Utilities|Array|MakeArray "ObjectTypeQuery3") false 0 "None"))
      (Utilities|Array|Clear (Variables|Default|GetHitActors))
      (for _array_element _outhits
        (bind _asbp_player (Utilities|Casting|CastToBP_Player (.HitActor (Collision|BreakHitResult _array_element))))
        (Utilities|Array|AddUnique (Variables|Default|GetHitActors) _asbp_player))
      ;[1 1 1] Apply Damage Radial
      (for _array_element_2 (Variables|Default|GetHitActors)
        (Utilities|IsValid _array_element_2
          (:Is%20Valid
            (Game|Damage|ApplyDamage _array_element_2 (Math|Float|MapRangeClamped (Math|Float|Absolute(Float) (Math|Vector|Distance(Vector) (Transformation|GetActorLocation _array_element_2) (.ImpactPoint (Collision|BreakHitResult (Variables|Default|GetHit))))) 0.0 _returnvalue 2e+01 2e+01) 0 0))))
      (Collision|SetCollisionEnabled (Variables|Default|GetSphere) "NoCollision"))))